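; BP_Door is the level exit door, locked until the referenced FeedMe object fires its ImFull event dispatcher.
; That event sets WinState, plays a buzzer and switches WinLight to the fulfilled material.
; Once won, interacting plays a latch sound, fades the camera out, then opens the WavesMainMenu level.
; Highlight and DeHighlight toggle custom depth on the handle, also only after the win.
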(event `self.ReceiveBeginPlay`
  (add `/Game/Gameplay/BP_Steven.ED_ImFull` (`self.FeedMeRef`) (delegate `ImFullEnd`)))

(event `ImFullEnd`
  (`GameplayStatics.PlaySoundAtLocation` "/Game/Sound/SFX/SC_DoorBuzzer_Cue.SC_DoorBuzzer_Cue" (`SceneComponent.K2_GetComponentLocation` (`self.WinLight`)) (struct) 1.0 1.0 0.0 "/Game/Sound/SFX/SA_RoomSounds.SA_RoomSounds" null null null)
  (set `self.WinState` true)
  (`PrimitiveComponent.SetMaterial` (`self.WinLight`) 0 "/Game/Art/Meshes/M_Dispenser/M_ButtonFulfilled.M_ButtonFulfilled"))

(event `/Game/Core/BPI_Interact.Interact`
  (params (Component :type "PrimitiveComponent Object Reference"))
  (if (`self.WinState`)
    (`GameplayStatics.PlaySoundAtLocation` "/Game/Sound/SFX/SC_door_latch1_Cue.SC_door_latch1_Cue" (`SceneComponent.K2_GetComponentLocation` (`self.Door`)) (struct) 1.0 1.0 0.0 null null null null)
    (`PlayerCameraManager.StartCameraFade` :`self` (`GameplayStatics.GetPlayerCameraManager` 0) :`ToAlpha` 1.0 :`Duration` 0.5 :`bHoldWhenFinished` true)
    (`KismetSystemLibrary.Delay` 2.0)
    (`GameplayStatics.OpenLevelBySoftObjectPtr` "/Game/wavesMainMenu.wavesMainMenu")))

(event `/Game/Core/BPI_Interact.Highlight`
  (params (Component :type "PrimitiveComponent Object Reference (by ref)"))
  (if (`self.WinState`)
    (if (== Component (`self.DoorHandle`))
      (`PrimitiveComponent.SetRenderCustomDepth` (`self.DoorHandle`) true))))

(event `/Game/Core/BPI_Interact.DeHighlight`
  (params (Component :type "PrimitiveComponent Object Reference (by ref)"))
  (if (`self.WinState`)
    (if (not (== Component (`self.DoorHandle`)))
      (`PrimitiveComponent.SetRenderCustomDepth` (`self.DoorHandle`) false))))

(fn `UserConstructionScript`)