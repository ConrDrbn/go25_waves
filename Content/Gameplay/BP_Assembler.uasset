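; BP_Assembler is an interactable machine with a button that spawns an item once.
; Interact on the button hit component spawns Item at the Spawner, sets Fulfilled and locks in the fulfilled material.
; Highlight and DeHighlight swap hover and idle materials until fulfilled.
; Left and right trigger boxes destroy their designated intake actors on overlap, without gating the spawn.
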(event `/Game/Core/BPI_Interact.Highlight`
  (params (Component :type "PrimitiveComponent Object Reference (by ref)"))
  (if (not (`self.Fulfilled`))
    (`/Engine/EditorBlueprintResources/StandardMacros.IsValid` Component
      (:`Is Valid`
        (if (== Component (`self.ButtonHit`))
          (`PrimitiveComponent.SetMaterial` (`self.Assembler_Button`) 0 "/Game/Art/Meshes/M_Dispenser/M_ButtonHighlight.M_ButtonHighlight"))))))

(event `/Game/Core/BPI_Interact.DeHighlight`
  (params (Component :type "PrimitiveComponent Object Reference (by ref)"))
  (if (not (`self.Fulfilled`))
    (`/Engine/EditorBlueprintResources/StandardMacros.IsValid` Component
      (:`Is Not Valid`
        (if (not (== Component (`self.ButtonHit`)))
          (`PrimitiveComponent.SetMaterial` (`self.Assembler_Button`) 0 "/Game/Art/Meshes/M_Dispenser/M_ButtonIdle.M_ButtonIdle"))))))

(event `/Game/Core/BPI_Interact.Interact`
  (params (Component :type "PrimitiveComponent Object Reference"))
  (`/Engine/EditorBlueprintResources/StandardMacros.IsValid` Component
    (:`Is Valid`
      (if (== Component (`self.ButtonHit`))
        (if (not (`self.Fulfilled`))
          (`|SpawnActorFromClass` (`self.Item`) (`KismetMathLibrary.MakeTransform` (`SceneComponent.K2_GetComponentLocation` (`self.Spawner`))) "AlwaysSpawn" "MultiplyWithRoot" null null)
          (set `self.Fulfilled` true)
          (`PrimitiveComponent.SetMaterial` (`self.Assembler_Button`) 0 "/Game/Art/Meshes/M_Dispenser/M_ButtonFulfilled.M_ButtonFulfilled"))))))

(event `self.BoxRight.OnComponentBeginOverlap`
  (params (OverlappedComponent :type "PrimitiveComponent Object Reference") (OtherActor :type "Actor Object Reference") (OtherComp :type "PrimitiveComponent Object Reference") (OtherBodyIndex :type Integer) (bFromSweep :type Boolean) (SweepResult :type "HitResult Structure (by ref)"))
  (if (== OtherActor (`self.RightIntake`))
    (`self.K2_DestroyActor` OtherActor)))

(event `self.BoxLeft.OnComponentBeginOverlap`
  (params (OverlappedComponent :type "PrimitiveComponent Object Reference") (OtherActor :type "Actor Object Reference") (OtherComp :type "PrimitiveComponent Object Reference") (OtherBodyIndex :type Integer) (bFromSweep :type Boolean) (SweepResult :type "HitResult Structure (by ref)"))
  (if (== OtherActor (`self.LeftIntake`))
    (`self.K2_DestroyActor` OtherActor)))

(fn `UserConstructionScript`)