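; BP_Steven is a customer-like actor that requests two or three random item classes and accepts them when they touch its sphere.
; BeginPlay moves random picks from ItemArray into ReqsArray and shows them on three planes through dynamic materials, using icon UV positions from DT_ItemIcons.
; A matching overlap plays an eating sound, then destroys the item after a delay; mismatches play a refusal.
; Emptying the list sets Fullfilled and calls the ImFull dispatcher.
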(event `self.ReceiveBeginPlay`
  (bind _plane1 (`self.Plane1`))
  (bind _plane2 (`self.Plane2`))
  (bind _plane (`self.Plane`))
  (`|ExecutionSequence`
    (:`then_0`
      (for _ (range 1 (+ (`KismetMathLibrary.RandomIntegerInRange` 2 3) 1))
        (bind _returnvalue (`KismetMathLibrary.RandomIntegerInRange` 0 12))
        (bind _output (`|GetArrayItem` (`self.ItemArray`) _returnvalue))
        (bind _returnvalue_2 (`KismetArrayLibrary.Array_Add` (`self.ReqsArray`) _output))
        (`KismetArrayLibrary.Array_RemoveItem` (`self.ItemArray`) _output)))
    (:`then_1`
      (bind _returnvalue_3 (`PrimitiveComponent.CreateDynamicMaterialInstance` _plane 0 (`PrimitiveComponent.GetMaterial` _plane 0) "None"))
      (bind _returnvalue_4 (`|GetDataTableRow` "/Game/UI/DT_ItemIcons.DT_ItemIcons" (`KismetStringLibrary.Conv_StringToName` (`KismetSystemLibrary.GetClassDisplayName` (`|GetArrayItem` (`self.ReqsArray`)))))
        (:`then`
          (`MaterialInstanceDynamic.SetVectorParameterValue` _returnvalue_3 "UVPos" (`.Address_8_1805687F456F46A82199D796B66B41A8` (break `/Game/UI/S_ItemIcons` _returnvalue_4))))))
    (:`then_2`
      (bind _returnvalue_5 (`PrimitiveComponent.CreateDynamicMaterialInstance` _plane1 0 (`PrimitiveComponent.GetMaterial` _plane1 0) "None"))
      (bind _returnvalue_6 (`|GetDataTableRow` "/Game/UI/DT_ItemIcons.DT_ItemIcons" (`KismetStringLibrary.Conv_StringToName` (`KismetSystemLibrary.GetClassDisplayName` (`|GetArrayItem` (`self.ReqsArray`) 1))))
        (:`then`
          (`MaterialInstanceDynamic.SetVectorParameterValue` _returnvalue_5 "UVPos" (`.Address_8_1805687F456F46A82199D796B66B41A8` (break `/Game/UI/S_ItemIcons` _returnvalue_6))))))
    (:`then_3`
      (bind _returnvalue_7 (`PrimitiveComponent.CreateDynamicMaterialInstance` _plane2 0 (`PrimitiveComponent.GetMaterial` _plane2 0) "None"))
      (bind _returnvalue_8 (`|GetDataTableRow` "/Game/UI/DT_ItemIcons.DT_ItemIcons" (`KismetStringLibrary.Conv_StringToName` (`KismetSystemLibrary.GetClassDisplayName` (`|GetArrayItem` (`self.ReqsArray`) 2))))
        (:`then`
          (`MaterialInstanceDynamic.SetVectorParameterValue` _returnvalue_7 "UVPos" (`.Address_8_1805687F456F46A82199D796B66B41A8` (break `/Game/UI/S_ItemIcons` _returnvalue_8))))))))

(event `self.Sphere.OnComponentBeginOverlap`
  (params (OverlappedComponent :type "PrimitiveComponent Object Reference") (OtherActor :type "Actor Object Reference") (OtherComp :type "PrimitiveComponent Object Reference") (OtherBodyIndex :type Integer) (bFromSweep :type Boolean) (SweepResult :type "HitResult Structure (by ref)"))
  (bind _returnvalue (`GameplayStatics.GetObjectClass` OtherActor))
  (if (not (`self.Fullfilled`))
    (for _array_element (`self.ReqsArray`)
      (if (== _array_element _returnvalue)
        (`KismetArrayLibrary.Array_RemoveItem` (`self.ReqsArray`) _returnvalue)
        (set `self.Success` true)))
    (if (`self.Success`)
      (`GameplayStatics.SpawnSoundAtLocation` "/Game/Sound/SFX/SC_sandwicheat09_Cue.SC_sandwicheat09_Cue" (`SceneComponent.K2_GetComponentLocation` (`self.StaticMesh`)) (struct) 1.0 1.0 0.0 null null)
      (`KismetSystemLibrary.Delay` 2.0)
      (`self.K2_DestroyActor` OtherActor)
      (if (== (`KismetArrayLibrary.Array_Length` (`self.ReqsArray`)) 0)
        (set `self.Fullfilled` true)
        (`GameplayStatics.SpawnSoundAtLocation` "/Game/Sound/SFX/SC_heavy_goodjob03_Cue.SC_heavy_goodjob03_Cue" (`SceneComponent.K2_GetComponentLocation` (`self.StaticMesh`)) (struct) 1.0 1.0 0.0 null null)
        (`self.ED_ImFull`)
        (set `self.Success` false))
      (else
        (`GameplayStatics.SpawnSoundAtLocation` "/Game/Sound/SFX/SC_heavy_no02_Cue.SC_heavy_no02_Cue" (`SceneComponent.K2_GetComponentLocation` (`self.StaticMesh`)) (struct) 1.0 1.0 0.0 null null)
        (set `self.Success` false)))))

(fn `UserConstructionScript`)