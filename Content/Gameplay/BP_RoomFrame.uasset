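; BP_RoomFrame is a timed room frame that travels via InterpToMovement and runs a fail countdown for the room.
; On BeginPlay it waits a configurable delay, plays a start sound, then moves toward TravelHeight as looping-motion audio fades in.
; The construction script sets movement duration from Timer, which also times the audio stop.
; A fixed delay of about two minutes then prints a failure message and fires the room-finished dispatcher.
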(event `self.ReceiveBeginPlay`
  (`MovementComponent.StopMovementImmediately` (`self.InterpToMovement`))
  (`AudioComponent.FadeOut` (`self.Audio`) 0.0 0.0 "Linear")
  (`KismetSystemLibrary.Delay` (`self.TimerDelay`))
  (`GameplayStatics.PlaySound2D` "/Game/Sound/SFX/SW_RoomStart.SW_RoomStart" 1.0 2.0 0.0 null null false)
  (`KismetSystemLibrary.Delay` 1.5)
  (`InterpToMovementComponent.AddControlPointPosition` (`self.InterpToMovement`) (`KismetMathLibrary.MakeVector` 0.0 0.0 (`self.TravelHeight`)) true)
  (`InterpToMovementComponent.RestartMovement` (`self.InterpToMovement`) 1.0)
  (`AudioComponent.FadeIn` (`self.Audio`) 0.5 0.2 0.0 "SCurve")
  (`KismetSystemLibrary.Delay` (`self.Timer`))
  (`AudioComponent.Stop` (`self.Audio`))
  (`self.FailTimer`))

(event `FailTimer`
  (`KismetSystemLibrary.Delay` 118.5)
  (`KismetSystemLibrary.PrintString` "You Failed!")
  (`self.ED_RoomFinished`))

(fn `UserConstructionScript`
  (set `InterpToMovementComponent.Duration` (`self.Timer`) (`self.InterpToMovement`)))