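; BP_IOPoint_New is an interactable item exchange point with Input, Output and Tribute types and a highlight decal.
; Input consumes the player's held item if it matches InputRef's OutputItem, then marks itself fulfilled.
; Output spawns its item once, optionally waiting until all Reqs are fulfilled.
; Tribute consumes items matching ManyInputsList and prints completion when all entries are fulfilled, but never sets their flags itself.
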(event `self.ReceiveBeginPlay`
  (bind _asbp_player (cast `/Game/Player/BP_Player` (`GameplayStatics.GetPlayerCharacter` 0)))
  (set `self.PlayerRef` _asbp_player))

(event `self.Highlight`
  (`SceneComponent.SetVisibility` (`self.Decal`) true false))

(event `self.DeHighlight`
  (`SceneComponent.SetVisibility` (`self.Decal`) false false))

(event `self.Interact`
  (bind _playerref (`self.PlayerRef`))
  (bind _playerref_2 (`self.PlayerRef`))
  (switch `/Game/Gameplay/E_IOPoint` (`self.Type`)
    (:`NewEnumerator0`
      (if (== (`/Game/Player/BP_Player.Item Ref` (`self.PlayerRef`)) (`/Game/Gameplay/BP_IOPoint.OutputItem` (`self.InputRef`)))
        (set `/Game/Player/BP_Player.Item Ref` null _playerref)
        (`StaticMeshComponent.SetStaticMesh` (`/Game/Player/BP_Player.ItemSlot` _playerref) null)
        (set `self.Fulfilled` true)))
    (:`NewEnumerator1`
      (if (`self.Fulfilled`)
        _
        (elif (`self.NeedReqs`)
          (for _array_element (`self.Reqs`)
            (set `self.Fulfilled` (`/Game/Gameplay/BP_IOPoint.Fulfilled` _array_element))
            (if (not (`self.Fulfilled`))
              (break)))
          (if (`self.Fulfilled`)
            (`|SpawnActorFromClass` (`self.OutputItem`) (`self.GetTransform` (`self.OutputSpawn`)) "AlwaysSpawn" "MultiplyWithRoot" null null :!label _label)
            (set `self.Fulfilled` true))
          (else
            (goto _label)))))
    (:`NewEnumerator2`
      (for _array_element_2 (`self.ManyInputsList`)
        (if (== (`/Game/Player/BP_Player.Item Ref` (`self.PlayerRef`)) (`/Game/Gameplay/BP_IOPoint.OutputItem` _array_element_2))
          (set `/Game/Player/BP_Player.Item Ref` null _playerref_2)
          (`StaticMeshComponent.SetStaticMesh` (`/Game/Player/BP_Player.ItemSlot` _playerref_2) null)
          (set `self.NumberFulfilled` 0)
          (for _array_element_3 (`self.ManyInputsList`)
            (if (== (`/Game/Gameplay/BP_IOPoint.Fulfilled` _array_element_3) true)
              (`/Engine/EditorBlueprintResources/StandardMacros.IncrementInt` (`self.NumberFulfilled`)
                (:`  `
                  (if (== (`self.NumberFulfilled`) (`KismetArrayLibrary.Array_Length` (`self.ManyInputsList`)))
                    (`KismetSystemLibrary.PrintString` "Tribute Complete!")))))))))))

(fn `UserConstructionScript`)