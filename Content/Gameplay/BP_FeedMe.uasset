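; BP_FeedMe is an actor that wants randomly chosen item classes fed to it through overlap.
; BeginPlay rolls one to three times into a unique requirement list, printing separately rolled names.
; FeedColl overlaps check the actor's class against the list, playing accept or reject sounds.
; Accepted actors are destroyed after a delay and the loop index, not necessarily the match, is removed; emptying the list calls CallEDImFull.
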(event `self.ReceiveBeginPlay`
  (bind _output (`|GetArrayItem` (`self.ItemArray`) (`KismetMathLibrary.RandomIntegerInRange` 0 12)))
  (for _ (range 1 (+ (`KismetMathLibrary.RandomIntegerInRange` 1 3) 1))
    (`KismetArrayLibrary.Array_AddUnique` (`self.ReqsArray`) _output)
    (`KismetSystemLibrary.PrintString` (`KismetSystemLibrary.GetClassDisplayName` _output) true true (struct :`G` 0.66 :`B` 1.0 :`A` 1.0) 500.0)))

(event `self.FeedColl.OnComponentBeginOverlap`
  (params (OverlappedComponent :type "PrimitiveComponent Object Reference") (OtherActor :type "Actor Object Reference") (OtherComp :type "PrimitiveComponent Object Reference") (OtherBodyIndex :type Integer) (bFromSweep :type Boolean) (SweepResult :type "HitResult Structure (by ref)"))
  (bind _returnvalue (`GameplayStatics.GetObjectClass` OtherActor))
  (bind _reqsarray (`self.ReqsArray`))
  (`KismetSystemLibrary.PrintString` (`KismetSystemLibrary.GetClassDisplayName` _returnvalue) true true (struct :`R` 1.0 :`G` 0.008229 :`A` 1.0))
  (if (not (`self.Fullfilled`))
    (for (_array_element _array_index) _reqsarray
      (set `self.Array Index` _array_index)
      (if (`KismetArrayLibrary.Array_Contains` _reqsarray _returnvalue)
        (`GameplayStatics.PlaySound2D` "/Game/Sound/SFX/SW_ButtonAccept.SW_ButtonAccept" 1.0 1.0 0.0 null null)
        (`KismetSystemLibrary.Delay` 2.0)
        (`self.K2_DestroyActor` OtherActor)
        (`KismetArrayLibrary.Array_Remove` (`self.ReqsArray`) (`self.Array Index`))
        (if (== (`KismetArrayLibrary.Array_Length` (`self.ReqsArray`)) 0)
          (set `self.Fullfilled` true)
          (`self.ED_ImFull`))
        (else
          (`GameplayStatics.PlaySound2D` "/Game/Sound/SFX/SW_ButtonReject.SW_ButtonReject" 1.0 1.0 0.0 null null)
          (break))))))

(fn `UserConstructionScript`)