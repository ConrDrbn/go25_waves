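; BP_DeathWave is a moving wave actor that plays an end sequence and returns the player to the waves menu.
; Its WaveMove event adds a relative control point along negative Y to an InterpToMovement component and restarts it.
; After a delay it fades the camera out, waits, then opens the WavesMenu level.
; The construction script sets the movement duration from a Timer variable.
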(event `WaveMove`
  (bind _interptomovement (`self.InterpToMovement`))
  (`InterpToMovementComponent.AddControlPointPosition` _interptomovement (0.0 -6000.0 0.0) true)
  (`InterpToMovementComponent.RestartMovement` _interptomovement 1.0)
  (`KismetSystemLibrary.Delay` 3.0)
  (`PlayerCameraManager.StartCameraFade` :`self` (`GameplayStatics.GetPlayerCameraManager` 0) :`ToAlpha` 1.0 :`Duration` 0.5 :`bHoldWhenFinished` true)
  (`KismetSystemLibrary.Delay` 2.0)
  (`GameplayStatics.OpenLevelBySoftObjectPtr` "/Game/wavesMenu.wavesMenu"))

(fn `UserConstructionScript`
  (set `InterpToMovementComponent.Duration` (`self.Timer`) (`self.InterpToMovement`)))