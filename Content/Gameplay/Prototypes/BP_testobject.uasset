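; BP_testobject is a prototype pickup that the player can highlight and interact with.
; It caches the player character as BP_Player on BeginPlay and toggles the mesh's custom depth render for highlighting.
; On interact, it copies its static mesh into the player's ItemSlot, passes its class to the player's ItemInfoMessage, then destroys itself.
; Custom depth stencil calls are present but unconnected.
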(event `self.ReceiveBeginPlay`
  (bind _asbp_player (cast `/Game/Player/BP_Player` (`GameplayStatics.GetPlayerCharacter` 0)))
  (set `self.PlayerRef` _asbp_player))

(event `/Game/Core/BPI_Interact.Highlight`
  (params (Component :type "PrimitiveComponent Object Reference (by ref)"))
  (`PrimitiveComponent.SetRenderCustomDepth` (`self.Mesh`) true))

(event `/Game/Core/BPI_Interact.DeHighlight`
  (params (Component :type "PrimitiveComponent Object Reference (by ref)"))
  (`PrimitiveComponent.SetRenderCustomDepth` (`self.Mesh`) false))

(event `/Game/Core/BPI_Interact.Interact`
  (params (Component :type "PrimitiveComponent Object Reference"))
  (`StaticMeshComponent.SetStaticMesh` (`/Game/Player/BP_Player.ItemSlot` (`self.PlayerRef`)) (`StaticMeshComponent.StaticMesh` (`self.Mesh`)))
  (message `/Game/Core/BPI_Player.ItemInfo` (`self.PlayerRef`) (`GameplayStatics.GetObjectClass` self))
  (`self.K2_DestroyActor`))

(fn `UserConstructionScript`)