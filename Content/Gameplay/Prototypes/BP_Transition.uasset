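; A prototype transition object that opens the WavesMenu level once the player meets a feeding win condition.
; On BeginPlay it binds to the FeedMe reference's "I'm full" event dispatcher, which sets a win flag, prints a message and swaps the WinLight material to fulfilled.
; Interact loads the level only after winning; the highlight events are empty stubs.
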(event `self.ReceiveBeginPlay`
  (add `/Game/Gameplay/BP_Steven.ED_ImFull` (`self.FeedMeRef`) (delegate `ImFullEnd`)))

(event `ImFullEnd`
  (`KismetSystemLibrary.PrintString` "You Live to Feed Another Day")
  (set `self.WinState` true)
  (`PrimitiveComponent.SetMaterial` (`self.WinLight`) 0 "/Game/Art/Meshes/M_Dispenser/M_ButtonFulfilled.M_ButtonFulfilled"))

(event `/Game/Core/BPI_Interact.Interact`
  (params (Component :type "PrimitiveComponent Object Reference"))
  (if (`self.WinState`)
    (`GameplayStatics.OpenLevelBySoftObjectPtr` "/Game/wavesMenu.wavesMenu")))

(event `/Game/Core/BPI_Interact.Highlight`
  (params (Component :type "PrimitiveComponent Object Reference (by ref)"))
  (if (`self.WinState`)
    _))

(event `/Game/Core/BPI_Interact.DeHighlight`
  (params (Component :type "PrimitiveComponent Object Reference (by ref)")))

(fn `UserConstructionScript`)