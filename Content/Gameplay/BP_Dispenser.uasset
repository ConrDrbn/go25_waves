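; A one-shot dispenser actor that spawns its configured Item class at the Spawner when its button is interacted with.
; Highlight and DeHighlight events swap the button material and custom depth, with a DoOnce limiting the highlight sound.
; Interact marks it fulfilled, locking out further use and highlighting.
; On BeginPlay, a dynamic screen material gets its icon UV position from DT_ItemIcons, keyed by the item's class display name.
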(event `/Game/Core/BPI_Interact.Highlight`
  (params (Component :type "PrimitiveComponent Object Reference (by ref)"))
  (bind _sm_dispenserbutton (`self.SM_DispenserButton`))
  (if (not (`self.Fulfilled`))
    (`/Engine/EditorBlueprintResources/StandardMacros.IsValid` Component
      (:`Is Valid`
        (if (== Component (`self.SM_DispenserButton`))
          (`PrimitiveComponent.SetMaterial` _sm_dispenserbutton 0 "/Game/Art/Meshes/M_Dispenser/M_ButtonHighlight.M_ButtonHighlight")
          (`PrimitiveComponent.SetRenderCustomDepth` _sm_dispenserbutton true)
          (`/Engine/EditorBlueprintResources/StandardMacros.DoOnce` false :!label _label
            (:`Completed`
              (`GameplayStatics.PlaySoundAtLocation` "/Game/Sound/SFX/SW_ButtonHighlight.SW_ButtonHighlight" (`SceneComponent.K2_GetComponentLocation` _sm_dispenserbutton) (struct) 1.0 1.0 0.0 null null null null))))))))

(event `/Game/Core/BPI_Interact.DeHighlight`
  (params (Component :type "PrimitiveComponent Object Reference (by ref)"))
  (bind _sm_dispenserbutton (`self.SM_DispenserButton`))
  (if (not (`self.Fulfilled`))
    (`/Engine/EditorBlueprintResources/StandardMacros.IsValid` Component
      (:`Is Not Valid`
        (if (not (== Component (`self.SM_DispenserButton`)))
          (`PrimitiveComponent.SetMaterial` _sm_dispenserbutton 0 "/Game/Art/Meshes/M_Dispenser/M_ButtonIdle.M_ButtonIdle")
          (`PrimitiveComponent.SetRenderCustomDepth` _sm_dispenserbutton false)
          (goto _label :!via `Reset`))))))

(event `/Game/Core/BPI_Interact.Interact`
  (params (Component :type "PrimitiveComponent Object Reference"))
  (bind _sm_dispenserbutton (`self.SM_DispenserButton`))
  (`/Engine/EditorBlueprintResources/StandardMacros.IsValid` Component
    (:`Is Valid`
      (if (== Component (`self.SM_DispenserButton`))
        (if (not (`self.Fulfilled`))
          (`|SpawnActorFromClass` (`self.Item`) (`KismetMathLibrary.MakeTransform` (`SceneComponent.K2_GetComponentLocation` (`self.Spawner`))) "AlwaysSpawn" "MultiplyWithRoot" null null)
          (set `self.Fulfilled` true)
          (`PrimitiveComponent.SetMaterial` _sm_dispenserbutton 0 "/Game/Art/Meshes/M_Dispenser/M_ButtonFulfilled.M_ButtonFulfilled")
          (`PrimitiveComponent.SetRenderCustomDepth` _sm_dispenserbutton false)
          (`GameplayStatics.PlaySoundAtLocation` "/Game/Sound/SFX/SW_ButtonAccept.SW_ButtonAccept" (`SceneComponent.K2_GetComponentLocation` _sm_dispenserbutton) (struct) 1.0 1.0 0.0 null null null null))))))

(event `self.ReceiveBeginPlay`
  (bind _sm_screenpanel (`self.SM_ScreenPanel`))
  (bind _returnvalue (`PrimitiveComponent.CreateDynamicMaterialInstance` _sm_screenpanel 0 (`PrimitiveComponent.GetMaterial` _sm_screenpanel 0) "None"))
  (set `self.MatRef` _returnvalue)
  (bind _returnvalue_2 (`|GetDataTableRow` "/Game/UI/DT_ItemIcons.DT_ItemIcons" (`KismetStringLibrary.Conv_StringToName` (`KismetSystemLibrary.GetClassDisplayName` (`self.Item`))))
    (:`then`
      (`MaterialInstanceDynamic.SetVectorParameterValue` (`self.MatRef`) "UVPos" (`.Address_8_1805687F456F46A82199D796B66B41A8` (break `/Game/UI/S_ItemIcons` _returnvalue_2))))
    (:`RowNotFound`
      (`KismetSystemLibrary.PrintString` "FailedRowCheck" true true (struct :`R` 1.0 :`G` 0.079728 :`A` 1.0) 10.0))))

(fn `UserConstructionScript`)