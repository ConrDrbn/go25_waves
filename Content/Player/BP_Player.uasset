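; BP_Player is the first-person player character, handling Enhanced Input movement, camera look and interaction with world objects.
; Each Tick, a sphere trace from the camera highlights BPI_Interact actors through interface messages and de-highlights the stored actor when none is hit.
; The Interact input repeats the trace and sends InteractMessage to the hit actor.
; BeginPlay adds the mapping context and sets game-only input, while helper functions apply look and movement.
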(event `self.ReceiveTick`
  (params (DeltaSeconds :type "Float (single-precision)"))
  (bind _camera (`self.Camera`))
  (bind _highlighted (`self.Highlighted`))
  (bind _returnvalue (`SceneComponent.K2_GetComponentLocation` _camera))
  (bind (_outhit _returnvalue_2) (`KismetSystemLibrary.SphereTraceSingle` _returnvalue (+ _returnvalue (* (`SceneComponent.GetForwardVector` _camera) (`self.ScanReach`))) 5.0 "TraceTypeQuery1"))
  (if _returnvalue_2
    (bind (_bblockinghit _binitialoverlap _time _distance _location _impactpoint _normal _impactnormal _physmat _hitactor) (`GameplayStatics.BreakHitResult` _outhit))
    (if (`KismetSystemLibrary.DoesImplementInterface` _hitactor "/Game/Core/BPI_Interact.BPI_Interact_C")
      (set `self.Highlighted` _hitactor)
      (message `/Game/Core/BPI_Interact.Highlight` _hitactor)
      (else
        (`/Engine/EditorBlueprintResources/StandardMacros.IsValid` _highlighted :!label _label
          (:`Is Valid`
            (message `/Game/Core/BPI_Interact.DeHighlight` _highlighted)))))
    (else
      (goto _label))))

(event `self.ReceiveBeginPlay`
  ; BeginPlay Setup
  (`self.AddInputMapping`)
  (`WidgetBlueprintLibrary.SetInputMode_GameOnly` (`GameplayStatics.GetPlayerController` 0)))

(event `AddInputMapping`
  ; Controls
  (`self.MappingContextScript` "/Game/Inputs/IMC_Player.IMC_Player"))

(event `EnhancedInput|/Game/Inputs/IA_Interact`
  (params (ActionValue :type Boolean) (ElapsedSeconds :type "Float (double-precision)") (TriggeredSeconds :type "Float (double-precision)") (InputAction :type "InputAction Object Reference" :default "/Game/Inputs/IA_Interact.IA_Interact"))
  (bind _camera (`self.Camera`))
  (bind _returnvalue (`SceneComponent.K2_GetComponentLocation` _camera))
  (:`Started`
    (bind _outhit (`KismetSystemLibrary.SphereTraceSingle` _returnvalue (+ _returnvalue (* (`SceneComponent.GetForwardVector` _camera) (`self.ScanReach`))) 5.0 "TraceTypeQuery1"))
    (bind (_bblockinghit _binitialoverlap _time _distance _location _impactpoint _normal _impactnormal _physmat _hitactor) (`GameplayStatics.BreakHitResult` _outhit))
    (if (`KismetSystemLibrary.DoesImplementInterface` _hitactor "/Game/Core/BPI_Interact.BPI_Interact_C")
      (message `/Game/Core/BPI_Interact.Interact` _hitactor))))

(event `EnhancedInput|/Game/Inputs/IA_Look`
  (params (ActionValue :type "Vector2D Structure") (ElapsedSeconds :type "Float (double-precision)") (TriggeredSeconds :type "Float (double-precision)") (InputAction :type "InputAction Object Reference" :default "/Game/Inputs/IA_Look.IA_Look"))
  ; Controls
  (:`Triggered`
    (`self.CameraLook` ActionValue_X ActionValue_Y (`self.Sensitivity`))))

(event `EnhancedInput|/Game/Inputs/IA_Move`
  (params (ActionValue :type "Vector2D Structure") (ElapsedSeconds :type "Float (double-precision)") (TriggeredSeconds :type "Float (double-precision)") (InputAction :type "InputAction Object Reference" :default "/Game/Inputs/IA_Move.IA_Move"))
  ; Controls
  (:`Triggered`
    (`self.Movement` ActionValue_X ActionValue_Y)))

(fn `CameraLook`
  (params (ValueX :type "Float (double-precision)") (ValueY :type "Float (double-precision)") (ValueSensitivity :type "Float (double-precision)"))
  (`self.AddControllerYawInput` (* ValueX ValueSensitivity)) ; Left / Right
  (`self.AddControllerPitchInput` (* ValueY ValueSensitivity)) ; Up / Down
)

(fn `MappingContextScript`
  (params (MappingContext :type "InputMappingContext Object Reference"))
  (bind _returnvalue (pcsubsystem `EnhancedInputLocalPlayerSubsystem` (`GameplayStatics.GetPlayerController` 0)))
  (`/Engine/EditorBlueprintResources/StandardMacros.IsValid` _returnvalue
    (:`Is Valid`
      (`EnhancedInputSubsystemInterface.AddMappingContext` _returnvalue MappingContext 0 (struct)))))

(fn `Movement`
  (params (ValueX :type "Float (double-precision)") (ValueY :type "Float (double-precision)"))
  (`self.AddMovementInput` (`SceneComponent.GetRightVector` (`self.Camera`)) ValueX) ; Left / Right
  (`self.AddMovementInput` (`SceneComponent.GetForwardVector` (`self.CapsuleComponent`)) ValueY) ; Forward / Backward
)

(fn `UserConstructionScript`)